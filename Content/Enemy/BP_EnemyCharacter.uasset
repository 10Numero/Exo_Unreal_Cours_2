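; Zombie enemy character that roams, chases and attacks the player, and dies when its health drops below zero.
; It registers itself with the player, then wanders to random navigable points until PawnSensing triggers a chase ending in an attack montage.
; A retriggerable delay returns it to roaming once sightings stop.
; GetHit subtracts health, while Tick polls it to flag the animation Blueprint's death state and destroy the actor after a delay.
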(event `self.ReceiveTick`
  (params (DeltaSeconds :type "Float (single-precision)"))
  ;[1 1 1] Death
  (`|ExecutionSequence`
    (:`then_0`
      (if (< (`self.health`) 0.0)
        (set `self.isDead` true)
        (`MovementComponent.StopMovementImmediately` (`self.CharacterMovement`))
        (bind _asenemy_animation_bp (cast `/Game/Enemy/EnemyAnimationBP` (`SkeletalMeshComponent.GetAnimInstance` (`self.Mesh`))))
        (set `/Game/Enemy/EnemyAnimationBP.isDead` true _asenemy_animation_bp)
        (`KismetSystemLibrary.Delay` 2.67)
        (`self.Death`)))))

(event `self.ReceiveBeginPlay`
  ;[1 1 1] Start Roam
  (`self.Roam`)
  (bind _asmixamo_third_person_character (cast `/Game/MixamoChar/Mixamo_ThirdPersonCharacter` (`GameplayStatics.GetPlayerCharacter` 0)))
  (set `/Game/MixamoChar/Mixamo_ThirdPersonCharacter.Enemy` self _asmixamo_third_person_character))

(event `Roam`
  ;[1 1 1] Roam
  (`|AIMoveTo` self (`NavigationSystemV1.K2_GetRandomLocationInNavigableRadius` (`self.K2_GetActorLocation`) 500.0 null null) null
    (:`OnSuccess`
      (if (not (`self.seeCharacter`))
        (`self.Roam`)))))

(event `self.PawnSensing.OnSeePawn`
  (params (Pawn :type "Pawn Object Reference"))
  ;[1 1 1] Roam
  (bind _asmixamo_third_person_character (cast `/Game/MixamoChar/Mixamo_ThirdPersonCharacter` Pawn))
  (`|ExecutionSequence`
    (:`then_0`
      (set `self.seeCharacter` true)
      (`|AIMoveTo` self (0.0 0.0 0.0) _asmixamo_third_person_character
        (:`OnSuccess`
          (`self.PlayAnimMontage` "/Game/Enemy/Zombie_Attack_Montage.Zombie_Attack_Montage"))))
    (:`then_1`
      (`KismetSystemLibrary.RetriggerableDelay` 3.0)
      (`KismetSystemLibrary.PrintString` "Enemy lost u")
      (set `self.seeCharacter` false)
      (`self.Roam`))))

(fn `Death`
  (`self.K2_DestroyActor`))

(fn `GetHit`
  (`KismetSystemLibrary.PrintString` "Enemy Getting Hit")
  (set `self.health` (- (`self.health`) 25.0))
  (if (< (`self.health`) 0.0)
    (set `self.isDead` true)
    (`MovementComponent.StopMovementImmediately` (`self.CharacterMovement`))
    (else
      (`self.PlayAnimMontage` "/Game/Enemy/AM_Hit.AM_Hit"))))

(fn `UserConstructionScript`)